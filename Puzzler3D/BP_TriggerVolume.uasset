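; BP_TriggerVolume is a goal trigger in Puzzler3D that sends the game to the WinMenu level when BP_Yin overlaps it.
; On BeginPlay it creates a dynamic material instance on its Cube.
; A BP_Yin overlap sets the Armed flag and the matching material parameter, then opens WinMenu immediately.
; A BP_EnemyYin overlap destroys that enemy only if the volume is already armed.
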(event Collision|EventActorBeginOverlap
  (params (OtherActor :type Actor%20Object%20Reference))
  (Utilities|Casting|CastToBP_Yin OtherActor
    (:then
      (Variables|Default|SetArmed true)
      (Rendering|Material|SetScalarParameterValue (Variables|Default|GetMaterialInstance) "Armed" 1.0 :!class /Script/Engine.MaterialInstanceDynamic)
      (Game|OpenLevel(byName) "/Game/Puzzler3D/WinMenu/WinMenu"))
    (:CastFailed
      (bind _asbp_enemy_yin (Utilities|Casting|CastToBP_EnemyYin OtherActor))
      (if (Variables|Default|GetArmed)
        (Actor|DestroyActor _asbp_enemy_yin)))))

(event EventBeginPlay
  (bind _returnvalue (Rendering|Material|CreateDynamicMaterialInstance (Variables|Default|GetCube) 0 0 "None" :!class /Script/Engine.PrimitiveComponent))
  (Variables|Default|SetMaterialInstance _returnvalue))

(fn ConstructionScript)